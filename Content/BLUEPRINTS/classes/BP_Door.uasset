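; BP_Door is a door that belongs to one of three groups set by DoorValue, with its material chosen per group in the construction script.
; Each of the three Activate events loops over every BP_Door in the level, turning the matching group 90 degrees and resetting all others to zero rotation.
; The rotation is instant, as the LerpRotator nodes have no alpha input or timeline driving them.
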(event EventActivate0
  (bind _outactors (Actor|GetAllActorsOfClass "BP_Door_C"))
  (for _array_element _outactors
    (if (== (Variables|BP_Door_C|GetdoorValue _array_element) 0)
      (Transformation|SetRelativeRotation (Variables|/Script/Engine.Actor|GetRootComponent _array_element) (Math|Rotator|Lerp(Rotator) "0.000000,90.000000,0.000000" "0, 0, 0" 0.0) false false)
      (else
        (Transformation|SetRelativeRotation (Variables|/Script/Engine.Actor|GetRootComponent _array_element) (Math|Rotator|Lerp(Rotator) "0, 0, 0" "0.000000,90.000000,0.000000" 0.0) false false)))))

(event EventActivate1
  (bind _outactors (Actor|GetAllActorsOfClass "BP_Door_C"))
  (for _array_element _outactors
    (if (== (Variables|BP_Door_C|GetdoorValue _array_element) 1)
      (Transformation|SetRelativeRotation (Variables|/Script/Engine.Actor|GetRootComponent _array_element) (Math|Rotator|Lerp(Rotator) "0.000000,90.000000,0.000000" "0, 0, 0" 0.0) false false)
      (else
        (Transformation|SetRelativeRotation (Variables|/Script/Engine.Actor|GetRootComponent _array_element) (Math|Rotator|Lerp(Rotator) "0, 0, 0" "0.000000,90.000000,0.000000" 0.0) false false)))))

(event EventActivate2
  (bind _outactors (Actor|GetAllActorsOfClass "BP_Door_C"))
  (for _array_element _outactors
    (if (== (Variables|BP_Door_C|GetdoorValue _array_element) 2)
      (Transformation|SetRelativeRotation (Variables|/Script/Engine.Actor|GetRootComponent _array_element) (Math|Rotator|Lerp(Rotator) "0.000000,90.000000,0.000000" "0, 0, 0" 0.0) false false)
      (else
        (Transformation|SetRelativeRotation (Variables|/Script/Engine.Actor|GetRootComponent _array_element) (Math|Rotator|Lerp(Rotator) "0, 0, 0" "0.000000,90.000000,0.000000" 0.0) false false)))))

(fn ConstructionScript
  (switch int (Variables|Default|GetdoorValue)
    (:0
      (Rendering|Material|SetMaterial (Variables|Default|Getdoor3) 0 "/Game/MATERIALS/DoorMaterial.DoorMaterial"))
    (:1
      (Rendering|Material|SetMaterial (Variables|Default|Getdoor3) 0 "/Game/MATERIALS/DoorMaterial1.DoorMaterial1"))
    (:2
      (Rendering|Material|SetMaterial (Variables|Default|Getdoor3) 0 "/Game/MATERIALS/DoorMaterial2.DoorMaterial2"))))