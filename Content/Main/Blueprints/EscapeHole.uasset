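; EscapeHole is an exit actor Blueprint, apparently meant to show a win screen once the player has collected cheese.
; Each Tick, it searches for all BP_MainVRpawn actors and copies the first one's CurrentCheese into its own variable.
; The collision overlap event is empty.
; The logic to create the win widget, check the cheese count and display it is disconnected, so it never runs.
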(event OnComponentBeginOverlap(Collision)
  (params (OverlappedComponent :type Primitive%20Component%20Object%20Reference) (OtherActor :type Actor%20Object%20Reference) (OtherComp :type Primitive%20Component%20Object%20Reference) (OtherBodyIndex :type Integer) (bFromSweep :type Boolean) (SweepResult :type Hit%20Result%20Structure%20%28by%20ref%29)))

(event EventBeginPlay)

(event Collision|EventActorBeginOverlap
  (params (OtherActor :type Actor%20Object%20Reference)))

(event EventTick
  (params (DeltaSeconds :type Float%20%28single-precision%29))
  (bind _outactors (Actor|GetAllActorsOfClass "/Game/Main/Characters/BP_MainVRpawn.BP_MainVRpawn_C"))
  (Variables|Default|SetCurrentCheese2 (Variables|/Game/Main/Characters/BP_MainVRpawn.BP_MainVRpawn_C|GetCurrentCheese (Utilities|Array|Get(acopy) _outactors))))

(fn ConstructionScript)