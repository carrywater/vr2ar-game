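; Procedural mesh generator Blueprint that builds mesh sections from authored point and triangle data in its Construction Script.
; Each Sections entry becomes one mesh section: point locations become vertices, rotation up vectors become normals, and triangle structs flatten into the index list.
; Despite its name, CreateRandomSection involves no randomness.
; A separate CreateTriangle helper, not called here, builds a triangle with its three indices sorted ascending.
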(fn ConstructionScript
  (for (_array_element _array_index) (Variables|Default|GetSections)
    (CallFunction|CreateRandomSection _array_element _array_index)))

(fn CreateRandomSection
  (params (SectionData :type S%20Procedural%20Mesh%20Section%20Structure) (SectionIndex :type Integer))
  (bind (_points _triangles) (Utilities|Struct|BreakS_ProceduralMeshSection SectionData))
  (bind _triangles_2 (LocalVariables|GetTriangles))
  (for _array_element _points
    (Utilities|Array|Add (LocalVariables|GetVertices) (.Location (Math|Transform|BreakTransform (Utilities|Struct|BreakS_ProceduralMeshPoint _array_element))))
    (Utilities|Array|Add (LocalVariables|GetNormals) (Math|Vector|GetUpVector (.Rotation (Math|Transform|BreakTransform (Utilities|Struct|BreakS_ProceduralMeshPoint _array_element))))))
  (for _array_element_2 _triangles
    (Utilities|Array|Add _triangles_2 (.Vertex1 (Utilities|Struct|BreakS_ProceduralMeshTriangle _array_element_2)))
    (Utilities|Array|Add _triangles_2 (.Vertex2 (Utilities|Struct|BreakS_ProceduralMeshTriangle _array_element_2)))
    (Utilities|Array|Add _triangles_2 (.Vertex3 (Utilities|Struct|BreakS_ProceduralMeshTriangle _array_element_2))))
  (Class|ProceduralMeshComponent|CreateMeshSectionLinearColor (Variables|Default|GetProceduralMesh) SectionIndex (LocalVariables|GetVertices) (LocalVariables|GetTriangles) (LocalVariables|GetNormals) 0 0 0 0 0 0 false false))

(fn CreateTriangle
  (params (V1 :type Integer) (V2 :type Integer) (V3 :type Integer))
  (bind _returnvalue (Math|Integer|Min(Integer) V1 V2 V3))
  (bind _returnvalue_2 (Math|Integer|Max(Integer) V1 V2 V3))
  (return (Utilities|Struct|MakeS_ProceduralMeshTriangle _returnvalue (Utilities|Operators|Subtract (+ V1 V2 V3) _returnvalue _returnvalue_2) _returnvalue_2)))