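; VR game mode that provides a function to scatter cheese pickups across the level's spawn points.
; SpawnItem gathers all SpawnPoint actors, then spawns MaxCheeseNeeded Cheeze actors at randomly chosen points, adjusting for collisions but always spawning.
; Each used point is removed from the list and destroyed, so no location repeats.
; The event graph is empty, and nothing in this Blueprint calls SpawnItem.
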(event EventBeginPlay)

(event EventTick
  (params (DeltaSeconds :type Float%20%28single-precision%29)))

(fn ConstructionScript)

(fn SpawnItem
  (bind _outactors (Actor|GetAllActorsOfClass "/Game/Kuba/Cheeze/SpawnPoint.SpawnPoint_C"))
  (LocalVariables|SetLocalSpawnReference _outactors)
  (for _index (range 0 (- (Variables|Default|GetMaxCheeseNeeded) 1))
    (Variables|Default|SetLocalItem (.OutItem (Utilities|Array|Random (LocalVariables|GetLocalSpawnReference))))
    (Game|SpawnActorfromClass "/Game/Kuba/Cheeze/Cheeze.Cheeze_C" (Math|Transform|MakeTransform (Transformation|GetActorLocation (Variables|Default|GetLocalItem))) "AdjustIfPossibleButAlwaysSpawn" "MultiplyWithRoot" 0 0)
    (Utilities|Array|RemoveItem (LocalVariables|GetLocalSpawnReference) (Variables|Default|GetLocalItem))
    (Actor|DestroyActor (Variables|Default|GetLocalItem))))