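; Spline-based patrol route actor for the RougeHuman AI enemy, serving world-space patrol points.
; GetSplinePointAsWorldPosition returns the location of the PatrolRoute spline point at the current PatrolPointIndex.
; IncreamentPatrol steps that index by Direction, ping-pong style, flipping forward at zero.
; The backward flip compares against point count minus negative one, so it triggers past the last valid index.
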(event Custom|IncreamentPatrol
  (bind _output_get (Variables|Default|SetPatrolPointIndex (+ (Variables|Default|GetPatrolPointIndex) (Variables|Default|GetDirection))))
  (if (== _output_get (- (Spline|GetNumberOfSplinePoints (Variables|Default|GetPatrolRoute)) -1))
    (Variables|Default|SetDirection -1)
    (elif (== (Variables|Default|GetPatrolPointIndex) 0)
      (Variables|Default|SetDirection 1))))

(fn ConstructionScript)

(fn GetSplinePointasWorldPosition
  (return (Spline|GetLocationatSplinePoint (Variables|Default|GetPatrolRoute) (Variables|Default|GetPatrolPointIndex) "World")))