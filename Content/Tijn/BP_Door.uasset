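; BP_Door is a color-coded door in one of three groups set by DoorValue, with the construction script picking the matching material.
; Activate0, Activate1 and Activate2 each switch to their group unless already open, looping over every BP_Door to yaw that group 90 degrees and swing the previously open group back.
; OpenValue and IsOpened on the called instance track the open group.
; Rotation snaps instantly; LerpRotator branches are unconnected.
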(event EventActivate0
  (switch int (Variables|Default|GetopenValue)
    (:Default
      _)
    (:1
      _)
    (:2
      _))
  (bind _outactors (Actor|GetAllActorsOfClass "BP_Door_C"))
  (for _array_element _outactors
    (if (== (Variables|BP_Door_C|GetdoorValue _array_element) 0)
      (Transformation|SetRelativeRotation (Variables|/Script/Engine.Actor|GetRootComponent _array_element) (Math|Rotator|MakeRotator 0.0 0.0 (+ (.yaw (Math|Conversions|RotationFromXVector (Math|Vector|GetForwardVector (Variables|/Script/Engine.Actor|GetRootComponent _array_element)))) 9e+01)) false false)
      (elif (== (Variables|BP_Door_C|GetdoorValue _array_element) (Variables|Default|GetopenValue))
        (if (Variables|Default|GetisOpened)
          (Transformation|SetRelativeRotation (Variables|/Script/Engine.Actor|GetRootComponent _array_element) (Math|Rotator|MakeRotator 0.0 0.0 (+ (.yaw (Math|Conversions|RotationFromXVector (Math|Vector|GetForwardVector (Variables|/Script/Engine.Actor|GetRootComponent _array_element)))) -9e+01)) false false)))))
  (Variables|Default|SetisOpened true)
  (Variables|Default|SetopenValue 0))

(event EventActivate1
  (switch int (Variables|Default|GetopenValue)
    (:Default
      _)
    (:0
      _)
    (:2
      _))
  (bind _outactors (Actor|GetAllActorsOfClass "BP_Door_C"))
  (for _array_element _outactors
    (if (== (Variables|BP_Door_C|GetdoorValue _array_element) 1)
      (Transformation|SetRelativeRotation (Variables|/Script/Engine.Actor|GetRootComponent _array_element) (Math|Rotator|MakeRotator 0.0 0.0 (+ (.yaw (Math|Conversions|RotationFromXVector (Math|Vector|GetForwardVector (Variables|/Script/Engine.Actor|GetRootComponent _array_element)))) 9e+01)) false false)
      (elif (== (Variables|BP_Door_C|GetdoorValue _array_element) (Variables|Default|GetopenValue))
        (if (Variables|Default|GetisOpened)
          (Transformation|SetRelativeRotation (Variables|/Script/Engine.Actor|GetRootComponent _array_element) (Math|Rotator|MakeRotator 0.0 0.0 (+ (.yaw (Math|Conversions|RotationFromXVector (Math|Vector|GetForwardVector (Variables|/Script/Engine.Actor|GetRootComponent _array_element)))) -9e+01)) false false)))))
  (Variables|Default|SetisOpened true)
  (Variables|Default|SetopenValue 1))

(event EventActivate2
  (switch int (Variables|Default|GetopenValue)
    (:Default
      _)
    (:0
      _)
    (:1
      _))
  (bind _outactors (Actor|GetAllActorsOfClass "BP_Door_C"))
  (for _array_element _outactors
    (if (== (Variables|BP_Door_C|GetdoorValue _array_element) 2)
      (Transformation|SetRelativeRotation (Variables|/Script/Engine.Actor|GetRootComponent _array_element) (Math|Rotator|MakeRotator 0.0 0.0 (+ (.yaw (Math|Conversions|RotationFromXVector (Math|Vector|GetForwardVector (Variables|/Script/Engine.Actor|GetRootComponent _array_element)))) 9e+01)) false false)
      (elif (== (Variables|BP_Door_C|GetdoorValue _array_element) (Variables|Default|GetopenValue))
        (if (Variables|Default|GetisOpened)
          (Transformation|SetRelativeRotation (Variables|/Script/Engine.Actor|GetRootComponent _array_element) (Math|Rotator|MakeRotator 0.0 0.0 (+ (.yaw (Math|Conversions|RotationFromXVector (Math|Vector|GetForwardVector (Variables|/Script/Engine.Actor|GetRootComponent _array_element)))) -9e+01)) false false)))))
  (Variables|Default|SetisOpened true)
  (Variables|Default|SetopenValue 2))

(fn ConstructionScript
  (switch int (Variables|Default|GetdoorValue)
    (:0
      (Rendering|Material|SetMaterial (Variables|Default|Getdoor3) 0 "/Game/Tijn/DoorMaterial.DoorMaterial"))
    (:1
      (Rendering|Material|SetMaterial (Variables|Default|Getdoor3) 0 "/Game/Tijn/DoorMaterial1.DoorMaterial1"))
    (:2
      (Rendering|Material|SetMaterial (Variables|Default|Getdoor3) 0 "/Game/Tijn/DoorMaterial2.DoorMaterial2"))))