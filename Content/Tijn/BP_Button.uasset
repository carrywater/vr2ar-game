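; BP_Button is an interactable button that signals a door according to its ButtonValue.
; On interact it calls the matching Activate message (0, 1 or 2) on the first BP_Door found, then briefly swaps to the pressed mesh.
; The construction script colour-codes the button by assigning one of three door materials from that value.
; Disconnected leftover chains loop over all doors comparing DoorValue and never run.
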(event EventOnInteract
  (params (InteractingPlayer :type Character%20Object%20Reference))
  (bind _returnvalue (Actor|GetActorOfClass "/Game/Tijn/BP_Door.BP_Door_C"))
  (switch int (Variables|Default|GetbuttonValue)
    (:0
      (Class|Button|Activate0(Message) _returnvalue))
    (:1
      (Class|Button|Activate1(Message) _returnvalue))
    (:2
      (Class|Button|Activate2(Message) _returnvalue)))
  (Components|StaticMesh|SetStaticMesh (Variables|Default|GetButtonUp) "/Game/Tijn/ButtonDown.ButtonDown")
  (Utilities|FlowControl|Delay 0.8)
  (Components|StaticMesh|SetStaticMesh (Variables|Default|GetButtonUp) "/Game/Tijn/ButtonUp.ButtonUp"))

(event EventDoor
  (params (Interactor :type Character%20Object%20Reference)))

(fn ConstructionScript
  (bind _buttonup (Variables|Default|GetButtonUp))
  (switch int (Variables|Default|GetbuttonValue)
    (:0
      (Rendering|Material|SetMaterial _buttonup 1 "/Game/Tijn/DoorMaterial.DoorMaterial"))
    (:1
      (Rendering|Material|SetMaterial _buttonup 1 "/Game/Tijn/DoorMaterial1.DoorMaterial1"))
    (:2
      (Rendering|Material|SetMaterial _buttonup 1 "/Game/Tijn/DoorMaterial2.DoorMaterial2"))))